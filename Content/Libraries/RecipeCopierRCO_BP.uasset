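; Remote call object for the Recipe Copier that applies copied recipes, overclocks and splitter rules to target buildables.
; setRecipe honors copy mode, checks the machine can produce the recipe and empties its inventories before switching.
; Overclocking trades power shards with the player's inventory, dropping refund overflow, and caps potential at the machine's current maximum.
; setRules replaces all programmable splitter rules but matches smart splitter rules by output index.
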(event Custom|moveItems
  (params (sourceInventoryComponent :type FG%20Inventory%20Component%20Object%20Reference) (targetInventoryComponent :type FG%20Inventory%20Component%20Object%20Reference) (item :type FG%20Item%20Descriptor%20Class%20Reference) (amount :type Integer) (dropExcess :type Boolean) (player :type FG%20Character%20Player%20Object%20Reference))
  (RecipeCopier|MoveItemsImpl sourceInventoryComponent targetInventoryComponent item amount dropExcess player))

(event Custom|setRules
  (params (splitterSmart :type FG%20Buildable%20Splitter%20Smart%20Object%20Reference) (selectedRules :type Array%20of%20Splitter%20Sort%20Rule%20Structures) (player :type FG%20Character%20Player%20Object%20Reference) (copier :type Equip%20Recipe%20Copier%20Object%20Reference))
  (RecipeCopier|SetRulesImpl splitterSmart selectedRules player)
  (Class|RecipeCopierEquipment|ClearTargets copier))

(event Custom|setRecipe
  (params (factory :type FG%20Buildable%20Factory%20Object%20Reference) (selectedRecipe :type FG%20Recipe%20Class%20Reference) (selectedOverclock :type Float%20%28single-precision%29) (player :type FG%20Character%20Player%20Object%20Reference) (copyMode :type ERecipeCopyMode%20Enum :default "RecipeOnly") (copier :type Equip%20Recipe%20Copier%20Object%20Reference))
  (RecipeCopier|SetRecipeImpl factory selectedRecipe selectedOverclock player copyMode)
  (Class|RecipeCopierEquipment|ClearTargets copier))

(fn MoveItemsImpl
  (params (sourceInventoryComponent :type FG%20Inventory%20Component%20Object%20Reference) (targetInventoryComponent :type FG%20Inventory%20Component%20Object%20Reference) (item :type FG%20Item%20Descriptor%20Class%20Reference) (amount :type Integer) (dropExcess :type Boolean) (player :type FG%20Character%20Player%20Object%20Reference))
  (bind _returnvalue (Class|FGInventoryLibrary|MakeInventoryItem item))
  (bind _returnvalue_2 (Class|FGItemDescriptor|GetItemName item))
  (bind _output_get (LocalVariables|SetactualAmount (Math|Integer|Min(Integer) (Class|FGInventoryComponent|GetNumItems sourceInventoryComponent item) amount)))
  (Utilities|FlowControl|Sequence
    (:then_0
      (bind _returnvalue_3 (Class|FGInventoryComponent|AddStack targetInventoryComponent (Class|FGInventoryLibrary|MakeInventoryStack _output_get _returnvalue) true))
      (RecipeCopier|LogInfoPrefixedRCO (Utilities|Text|FormatText "Added {amount} {item} to {inventory}" _output_get _returnvalue_2 (RecipeCopier|GetPathNameTextRCO targetInventoryComponent)) true))
    (:then_1
      (Class|FGInventoryComponent|Remove sourceInventoryComponent item _returnvalue_3)
      (RecipeCopier|LogInfoPrefixedRCO (Utilities|Text|FormatText "Removed {amount} {item} from {inventory}" _returnvalue_3 _returnvalue_2 (RecipeCopier|GetPathNameTextRCO sourceInventoryComponent)) true))
    (:then_2
      (if dropExcess
        (Class|FGItemPickupSpawnable|CreateItemDropsinCylinder sourceInventoryComponent (Utilities|Array|MakeArray (Class|FGInventoryLibrary|MakeInventoryStack (- _output_get _returnvalue_3) _returnvalue)) (Transformation|GetActorLocation player) 2e+02 (Utilities|Array|MakeArray) 0)
        (RecipeCopier|LogInfoPrefixedRCO (Utilities|Text|FormatText "Dropped {amount} {item}" (- _output_get _returnvalue_3) (Utilities|Text|ToText(String) (Utilities|GetClassDisplayName item))) true)))))

(fn SetRecipeImpl
  (params (targetFactory :type FG%20Buildable%20Factory%20Object%20Reference) (selectedRecipe :type FG%20Recipe%20Class%20Reference) (selectedOverclock :type Float%20%28single-precision%29) (player :type FG%20Character%20Player%20Object%20Reference) (copyMode :type ERecipeCopyMode%20Enum :default "RecipeOnly"))
  (bind _returnvalue (Class|FGBuildableFactory|GetPendingPotential targetFactory))
  (bind _returnvalue_2 (!= selectedOverclock _returnvalue))
  (RecipeCopier|LogInfoPrefixedRCO (Utilities|Text|FormatText "Set Recipe Impl: {manufacturer} / {recipe} / {overclock} / {player} / {copyMode}" (RecipeCopier|GetPathNameTextRCO targetFactory) (Class|FGRecipe|GetRecipeName selectedRecipe) selectedOverclock (RecipeCopier|GetPathNameTextRCO player) (Utilities|Text|ToText(String) (Utilities|String|EnumtoString copyMode))) true)
  (Utilities|FlowControl|Sequence
    (:then_0
      ;[1 1 1] Copy recipe
      (if (Utilities|IsValidClass selectedRecipe)
        (bind _asfgbuildable_manufacturer (Utilities|Casting|CastToFGBuildableManufacturer targetFactory))
        (if (and (Utilities|Select :Index copyMode :RecipeOnly (!= (Class|FGBuildableManufacturer|GetCurrentRecipe _asfgbuildable_manufacturer) selectedRecipe) :OverclockOnly false :RecipeAndOverclock (!= (Class|FGBuildableManufacturer|GetCurrentRecipe _asfgbuildable_manufacturer) selectedRecipe)) (CallFunction|CanProduceRecipe selectedRecipe _asfgbuildable_manufacturer))
          (Utilities|FlowControl|Sequence
            (:then_0
              (Class|FGBuildableManufacturer|MoveorDropInputInventory _asfgbuildable_manufacturer player))
            (:then_1
              (Class|FGBuildableManufacturer|MoveorDropOutputInventory _asfgbuildable_manufacturer player))
            (:then_2
              (Class|FGBuildableManufacturer|SetRecipe _asfgbuildable_manufacturer selectedRecipe))))))
    (:then_1
      ;[1 1 1] Should we copy the potential, too?
      (if (and (Utilities|Select :Index copyMode :RecipeOnly false :OverclockOnly _returnvalue_2 :RecipeAndOverclock _returnvalue_2) (> selectedOverclock 0.0))
        (|handlePotential)))))

(fn LogInfoPrefixedRCO
  (params (message :type Text) (enabled :type Boolean))
  (bind _self self)
  (if enabled
    (Class|BlueprintLoggingLibrary|LogWarning (Utilities|String|ToString(Text) (Utilities|Text|FormatText "RecipeCopier {path}: {message}" (RecipeCopier|GetPathNameTextRCO _self _self) message)))))

(fn GetPathNameTextRCO
  (params (object :type Object%20Object%20Reference))
  (return (Utilities|Text|ToText(String) (Class|KismetSystemLibrary|GetPathName object))))

(fn SetRulesImpl
  (params (splitterSmart :type FG%20Buildable%20Splitter%20Smart%20Object%20Reference) (selectedRules :type Array%20of%20Splitter%20Sort%20Rule%20Structures) (player :type FG%20Character%20Player%20Object%20Reference))
  (bind _i (LocalVariables|Geti))
  (bind _i_2 (LocalVariables|Geti))
  (RecipeCopier|LogInfoPrefixedRCO (Utilities|Text|FormatText "Set Rules Impl: {splitterSmart} / {amount} / {player}" (RecipeCopier|GetPathNameTextRCO splitterSmart) (Utilities|Array|Length selectedRules) (RecipeCopier|GetPathNameTextRCO player)) true)
  (bind _asbuild_conveyor_attachment_splitter_programmable (Utilities|Casting|CastToBuild_ConveyorAttachmentSplitterProgrammable splitterSmart)
    (:then
      ;[0.7195 1 0.7257] Programmable Splitters - remove all existing and add the new ones
      (while (> (Class|FGBuildableSplitterSmart|GetNumSortRules _asbuild_conveyor_attachment_splitter_programmable) 0)
        (Class|FGBuildableSplitterSmart|RemoveSortRuleat _asbuild_conveyor_attachment_splitter_programmable))
      (for _array_element selectedRules
        (Class|FGBuildableSplitterSmart|AddSortRule splitterSmart _array_element)))
    (:CastFailed
      ;[1 0.8357 0.5687] Smart Splitter - loop through existing rules and replace then for the matching rule by OutputIndex
      (while (> (Class|FGBuildableSplitterSmart|GetNumSortRules splitterSmart) _i_2)
        (bind _rule (RecipeCopier|GetFirstRulebyOutputIndex selectedRules (.OutputIndex (Utilities|Struct|BreakSplitterSortRule (Class|FGBuildableSplitterSmart|GetSortRuleat splitterSmart _i_2)))))
        (Class|FGBuildableSplitterSmart|SetSortRuleat splitterSmart _i _rule)
        (Math|Integer|IncrementInt _i)))))

(fn SetIndexedRule
  (params (outputIndex :type Integer) (rules :type Array%20of%20Splitter%20Sort%20Rule%20Structures) (splitterSmart :type FG%20Buildable%20Splitter%20Smart%20Object%20Reference))
  (while (and (< (LocalVariables|GetruleIndex) 0) (< (LocalVariables|Geti) (Class|FGBuildableSplitterSmart|GetNumSortRules splitterSmart)))
    (if (== outputIndex (.OutputIndex (Utilities|Struct|BreakSplitterSortRule (Class|FGBuildableSplitterSmart|GetSortRuleat splitterSmart (LocalVariables|Geti)))))
      (LocalVariables|SetruleIndex (LocalVariables|Geti))
      (else
        (Math|Integer|IncrementInt (LocalVariables|Geti)))))
  (if (>= (LocalVariables|GetruleIndex) 0)
    (bind (_array_element _array_index) (Utilities|Array|ForEachLoopwithBreak rules :!label _label)
      (:LoopBody
        (if (== outputIndex (.OutputIndex (Utilities|Struct|BreakSplitterSortRule _array_element)))
          (Class|FGBuildableSplitterSmart|SetSortRuleat splitterSmart (LocalVariables|GetruleIndex) _array_element)
          (goto _label Break)
          (else
            (LocalVariables|Seti (+ _array_index 1)))))
      (:Completed
        (if (== (LocalVariables|Geti) (Utilities|Array|Length rules))
          (Class|FGBuildableSplitterSmart|SetSortRuleat splitterSmart (LocalVariables|GetruleIndex) (Utilities|Struct|MakeSplitterSortRule 0 outputIndex)))))))

(fn GetFirstRulebyOutputIndex
  (params (rules :type Array%20of%20Splitter%20Sort%20Rule%20Structures) (outputIndex :type Integer))
  (for _array_element rules
    (if (== (Utilities|Struct|BreakSplitterSortRule _array_element) outputIndex)
      (return _array_element)))
  (return (Utilities|Struct|MakeSplitterSortRule outputIndex)))

(fn CanProduceRecipe
  (params (recipe :type FG%20Recipe%20Class%20Reference) (manufacturer :type FG%20Buildable%20Manufacturer%20Object%20Reference))
  (LocalVariables|SetmanufacturerClass (Utilities|GetClass manufacturer))
  (for _array_element (Class|FGRecipe|GetProducedin recipe)
    (if (Utilities|ClassIsChildOf (LocalVariables|GetmanufacturerClass) _array_element)
      (return true)))
  (return false))